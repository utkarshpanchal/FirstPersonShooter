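; Enemy character Blueprint that carries a gun, shoots on the EnemyShoot event, takes damage and dies.
; BeginPlay hides the mesh's weapon bone, attaches a spawned BP_Gun to WeaponSocket and binds damage handling.
; Damage goes to CompDamage, and CompDeath's dead flag triggers delayed destruction.
; Helpers cache the player, check its death and freeze movement during the shoot montage; muzzle flash is empty and scope overlap only prints.
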(event OnComponentBeginOverlap(CapsuleComponent)
  (params (OverlappedComponent :type Primitive%20Component%20Object%20Reference) (OtherActor :type Actor%20Object%20Reference) (OtherComp :type Primitive%20Component%20Object%20Reference) (OtherBodyIndex :type Integer) (bFromSweep :type Boolean) (SweepResult :type Hit%20Result%20Structure%20%28by%20ref%29))
  (Utilities|Casting|CastToBP_Scope OtherActor)
  (Development|PrintString "its scope"))

(event Custom|Enemy_RecivingDamage
  (params (DamagedActor :type Actor%20Object%20Reference) (Damage :type Float%20%28single-precision%29) (DamageType :type Damage%20Type%20Object%20Reference) (InstigatedBy :type Controller%20Object%20Reference) (DamageCauser :type Actor%20Object%20Reference))
  (Default|TakeDamage (Variables|Default|GetComp_Damage))
  (if (Variables|/Game/Component/Comp_Death.Comp_Death_C|GetIsDead? (Variables|Default|GetComp_Death))
    (Utilities|FlowControl|Delay 3.0)
    (Actor|DestroyActor)))

(event Custom|EnemyShoot
  (bind _weapon (Variables|Default|GetWeapon))
  (Utilities|IsValid _weapon
    (:Is%20Valid
      (Default|PullTrigger _weapon))))

(event EventBeginPlay
  (Utilities|FlowControl|Sequence
    (:then_0
      (Components|SkinnedMesh|HideBonebyName (Variables|Character|GetMesh) "weapon_r" "PBO_None")
      (bind _returnvalue (Game|SpawnActorfromClass "/Game/Blueprints/Weapons/BP_Gun.BP_Gun_C" (Transformation|GetActorTransform) "Undefined" 0 0))
      (Variables|Default|SetWeapon _returnvalue)
      (Transformation|AttachComponentToComponent (Variables|Default|GetWeapon) (Variables|Character|GetMesh) "WeaponSocket" "SnapToTarget" "SnapToTarget" "KeepRelative" true)
      (Actor|SetOwner (Variables|Default|GetWeapon) self))
    (:then_1
      (EventDispatchers|AssignOnTakeAnyDamage (delegate Custom|Enemy_RecivingDamage)))))

(fn ConstructionScript)

(fn GetPlayerReference
  (bind _asbp_fps_player (Utilities|Casting|CastToBP_FPS_Player (Game|Player|GetPlayerPawn 0)))
  (Variables|Default|SetPlayer _asbp_fps_player))

(fn SpawnMuzzleFlash)