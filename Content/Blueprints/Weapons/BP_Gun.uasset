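; BP_Gun is a weapon that fires at player pawn 0 and damages it, rather than firing along its aim direction.
; PullTrigger chains validity-gated steps: fire sound, muzzle flash at the socket, then a trace with hit particles, so a missing asset stops everything after it.
; The trace runs from the muzzle socket to the player's location, and damage applies only when it hits BP_FPS_Player.
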(event Custom|PullTrigger
  (bind _muzzleflash (Variables|Default|GetMuzzleFlash))
  (bind _skeletalmesh (Variables|Default|GetSkeletalMesh))
  (bind _hitparticles (Variables|Default|GetHitParticles))
  (bind _gunfiresound (Variables|Default|GetGunFireSound))
  (Utilities|IsPawnValid
    (:Is%20Valid
      (Utilities|IsValid _gunfiresound
        (:Is%20Valid
          (Audio|PlaySoundatLocation _gunfiresound (Transformation|GetActorLocation) "0, 0, 0" 1.0 1.0 0.0 0 0 0 0)
          (Utilities|IsValid _muzzleflash
            (:Is%20Valid
              (CallFunction|SpawnMuzzleFlash _muzzleflash (Transformation|GetSocketLocation _skeletalmesh "MuzzleFlashSocket") (Transformation|GetSocketRotation _skeletalmesh "MuzzleFlashSocket"))
              (bind _pawnreference (Utilities|IsPawnValid)
                (:Is%20Valid
                  (Utilities|IsValid _hitparticles
                    (:Is%20Valid
                      (bind _outhit (CallFunction|SpawnLineTraceandColiderBulletParticles (Transformation|GetSocketLocation (Variables|Default|GetSkeletalMesh) "MuzzleFlashSocket") (Transformation|GetActorLocation _pawnreference) "None" _hitparticles))
                      (bind _asbp_fps_player (Utilities|Casting|CastToBP_FPS_Player (.hitactor _outhit)))
                      (Game|Damage|ApplyDamage _asbp_fps_player 1.0 0 self))))))))))))

(fn ConstructionScript)

(fn NewFunction)